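; BP_AI_小怪01 is a minor AI monster that switches its flipbook sprite to match its movement along the X axis.
; Each Tick, the sign of X velocity selects the right or left walk animation and stores that facing in ERight.
; When velocity is zero, ERight selects the matching idle flipbook; movement with zero X leaves the current animation unchanged.
; The Blueprint contains no movement or decision logic.
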(event EventBeginPlay)

(event Collision|EventActorBeginOverlap
  (params (OtherActor :type Actor%20Object%20Reference)))

(event EventTick
  (params (DeltaSeconds :type Float%20%28single-precision%29))
  (bind _returnvalue (Transformation|GetVelocity))
  (Math|Float|CompareFloat (.X (Math|Vector|BreakVector _returnvalue)) 0.0
    (:>
      (Sprite|SetFlipbook (Variables|Default|GetSprite) "/Game/素材库/AI/R_WALK.R_WALK")
      (Variables|Default|SetE_Right "NewEnumerator3"))
    (:==
      (if (not (> (Math|Vector|VectorLength _returnvalue) 0.0))
        (switch Utilities|FlowControl|Switch|SwitchonE_Right (Variables|Default|GetE_Right)
          (:NewEnumerator0
            (Sprite|SetFlipbook (Variables|Default|GetSprite) "/Game/素材库/AI/R_IDLE.R_IDLE")
            (Variables|Default|SetE_Right "NewEnumerator3"))
          (:NewEnumerator1
            (Sprite|SetFlipbook (Variables|Default|GetSprite) "/Game/素材库/AI/L_IDLE.L_IDLE")
            (Variables|Default|SetE_Right "NewEnumerator2")))))
    (:<
      (Sprite|SetFlipbook (Variables|Default|GetSprite) "/Game/素材库/AI/L_WALK.L_WALK")
      (Variables|Default|SetE_Right "NewEnumerator2"))))

(fn ConstructionScript)