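; Paper2D player character Blueprint with four-directional movement and idle, walk and run flipbook animations.
; MoveForward and MoveRight axes move it along world Y and X and record the facing direction, while the RUN action toggles max walk speed.
; Tick derives the movement state from velocity magnitude, then calls one of four per-direction functions (动作 to 动作_4) that set the matching Sprite flipbook.
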(event EventBeginPlay)

(event Collision|EventActorBeginOverlap
  (params (OtherActor :type Actor%20Object%20Reference)))

(event EventTick
  (params (DeltaSeconds :type Float%20%28single-precision%29))
  (bind _returnvalue (Transformation|GetVelocity))
  (bind _returnvalue_2 (Math|Vector|VectorLength _returnvalue))
  (Utilities|FlowControl|Sequence
    (:then_0
      (if (== _returnvalue_2 0.0)
        (Variables|Default|SetE_状态 "NewEnumerator0")
        (elif (>= _returnvalue_2 1.5e+02)
          (Variables|Default|SetE_状态 "NewEnumerator2")
          (else
            (Variables|Default|SetE_状态 "NewEnumerator1")))))
    (:then_1
      (switch Utilities|FlowControl|Switch|SwitchonE_Right (Variables|Default|GetE_Right)
        (:NewEnumerator0
          (|动作))
        (:NewEnumerator1
          (|动作_2))
        (:NewEnumerator2
          (|动作_3))
        (:NewEnumerator3
          (|动作_4))))))

(event Input|ActionEvents|InputActionRUN
  (params (Key :type Key%20Structure :default "None"))
  (bind _charactermovement (Variables|Character|GetCharacterMovement))
  (:Pressed
    (Variables|/Script/Engine.CharacterMovementComponent|SetMaxWalkSpeed _charactermovement 6e+02))
  (:Released
    (Variables|/Script/Engine.CharacterMovementComponent|SetMaxWalkSpeed _charactermovement 1.4e+02)))

(event Input|AxisEvents|InputAxisMoveForward
  (params (AxisValue :type Float%20%28single-precision%29))
  (Pawn|Input|AddMovementInput (Math|Vector|MakeVector 0.0 AxisValue 0.0) 1.0 false)
  (Math|Float|CompareFloat AxisValue 0.0
    (:>
      (Variables|Default|SetE_Right "NewEnumerator1"))
    (:<
      (Variables|Default|SetE_Right "NewEnumerator0"))))

(event Input|AxisEvents|InputAxisMoveRight
  (params (AxisValue :type Float%20%28single-precision%29))
  (Pawn|Input|AddMovementInput (Math|Vector|MakeVector AxisValue 0.0 0.0) 1.0 false)
  (Math|Float|CompareFloat AxisValue 0.0
    (:>
      (Variables|Default|SetE_Right "NewEnumerator3"))
    (:<
      (Variables|Default|SetE_Right "NewEnumerator2"))))

(fn ConstructionScript)